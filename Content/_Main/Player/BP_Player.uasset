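; Player character Blueprint handling movement, camera lock-on, rolling, sprinting, melee attacks and the pause menu.
; BPTargetingSystem handles lock-on input, while LockCamera stores the target that Turn input then faces the camera toward.
; Rolls and weak attacks run through server and multicast montage events; strong attack and blocking only print.
; Tick derives sprint from world X velocity, setting walk speed with server sync and an OnRep animation update.
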(event `self.ReceiveBeginPlay`
  ;[1 1 1] Target system
  (`/Game/_Main/Player/BP_TargetingSystem.Initialize` (`self.BP_TargetingSystem`)))

(event `InputAction|TargetLock`
  (params (Key :type "Key Structure"))
  ;[1 1 1] Target system
  (:`Pressed`
    (`/Game/_Main/Player/BP_TargetingSystem.LockOnTarget` (`self.BP_TargetingSystem`))))

(event `/Game/_Main/Interfaces/BPI_PlayerAnimBP.LockCamera`
  (params (LockCameraa :type Boolean) (Target :type "Actor Object Reference"))
  ;[1 1 1] Target system
  (bind _output_get (set `self.LockedOn` LockCameraa))
  (if _output_get
    (set `self.Target` Target)
    (else
      (set `self.Target` null))))

(event `InputAxis|Turn`
  (params (AxisValue :type "Float (single-precision)"))
  ;[1 1 1] Movement
  (if (not (`self.LockedOn`))
    (`self.AddControllerYawInput` AxisValue)
    (else
      (`self.f_LockOn`))))

(event `InputAxis|LookUp`
  (params (AxisValue :type "Float (single-precision)"))
  ;[1 1 1] Movement
  (if (not (`self.LockedOn`))
    (`self.AddControllerPitchInput` AxisValue)))

(event `InputAction|Rolling`
  (params (Key :type "Key Structure"))
  ;[1 1 1] Rolling Movement
  (:`Pressed`
    (if (not (`self.Rolling`))
      (`self.ServerRolling` true))))

(event `Server_ToggleSprint`
  (params (State :type Boolean))
  ;[1 1 1] Sprinting
  (`self.f_SprintSwitch` State))

(event `InputAxis|MoveForward`
  (params (AxisValue :type "Float (single-precision)"))
  ;[1 1 1] Movement
  (`self.AddMovementInput` (`KismetMathLibrary.GetForwardVector` (`KismetMathLibrary.MakeRotator` 0.0 0.0 (.yaw (`self.GetControlRotation`)))) AxisValue))

(event `self.ReceiveTick`
  (params (DeltaSeconds :type "Float (single-precision)"))
  (bind _returnvalue_x (`KismetMathLibrary.BreakVector` (`self.GetVelocity`)))
  ;[1 1 1] Sprinting
  (if (or (< _returnvalue_x -300.0) (> _returnvalue_x 300.0))
    (`self.f_SprintSwitch` true)
    (else
      (`self.f_SprintSwitch` false))))

(event `ServerRolling`
  (params (Rolling :type Boolean))
  ;[1 1 1] Rolling Movement
  (if Rolling
    (set `self.Rolling` true)
    (`self.MultiRolling` true (`self.Mesh`) "/Game/_Main/Player/PlayerRoll_Montage.PlayerRoll_Montage")
    (else
      (set `self.Rolling` false)
      (`self.MultiRolling` false null "/Game/_Main/Player/PlayerRoll_Montage.PlayerRoll_Montage"))))

(event `InputAxis|MoveRight`
  (params (AxisValue :type "Float (single-precision)"))
  ;[1 1 1] Movement
  (`self.AddMovementInput` (`KismetMathLibrary.GetRightVector` (`KismetMathLibrary.MakeRotator` 0.0 0.0 (.yaw (`self.GetControlRotation`)))) AxisValue))

(event `MultiRolling`
  (params (State :type Boolean) (Mesh :type "SkeletalMeshComponent Object Reference") (AnimMontage :type "AnimMontage Object Reference"))
  (bind _returnvalue (`SkeletalMeshComponent.GetAnimInstance` (`self.Mesh`)))
  ;[1 1 1] Rolling Movement
  (if State
    (message `/Game/_Main/Interfaces/BPI_PlayerAnimBP.RollingState` _returnvalue true)
    (else
      (message `/Game/_Main/Interfaces/BPI_PlayerAnimBP.RollingState` _returnvalue false)))
  (`|PlayMontage` Mesh AnimMontage
    (:`OnCompleted`
      (`self.ServerRolling` false))))

(event `InputAction|WeakAttack`
  (params (Key :type "Key Structure"))
  ;[1 1 1] Attack movement
  (:`Pressed`
    (`self.Server_TryToAttack` "NewEnumerator0")))

(event `InputAction|StrongAttack`
  (params (Key :type "Key Structure"))
  ;[1 1 1] Attack movement
  (:`Pressed`
    (`KismetSystemLibrary.PrintString` "Strong Attack")))

(event `InputAction|Blocking`
  (params (Key :type "Key Structure"))
  ;[1 1 1] Attack movement
  (:`Pressed`
    (`KismetSystemLibrary.PrintString` "Blocking")))

(event `Server_TryToAttack`
  (params (Attacks :type "/Game/_Main/Player/EnumPlayerAttacks Enum" :default "NewEnumerator0"))
  ;[1 1 1] Attack movement
  (if (and (not (`self.isAttacking`)) (not (`self.Rolling`)) (not (`self.IsBlocking`)))
    (switch `/Game/_Main/Player/EnumPlayerAttacks` Attacks
      (:`NewEnumerator0`
        (set `self.isAttacking` true)
        (`self.MultiAnimMontage` (`self.Mesh`) "/Game/_Main/Player/WeakAttackMontage.WeakAttackMontage")))))

(event `MultiAnimMontage`
  (params (InSkeletalMeshComponent :type "SkeletalMeshComponent Object Reference") (MontageToPlay :type "AnimMontage Object Reference") (StartingSection :type Name))
  ;[1 1 1] Attack movement
  (`|PlayMontage` InSkeletalMeshComponent MontageToPlay 1.0 0.0 StartingSection
    (:`OnCompleted`
      (`self.Server_EndAttack`))))

(event `Server_EndAttack`
  ;[1 1 1] Attack movement
  (set `self.isAttacking` false))

(event `InputAction|Pause`
  (params (Key :type "Key Structure"))
  ;[1 1 1] Pause Menu Creation on Button press
  (:`Pressed`
    (`GameplayStatics.SetGamePaused` true)
    (bind _returnvalue (`|CreateWidget` "/Game/_Main/Menus/PauseMenu.PauseMenu_C"))
    (bind _output_get (set `self.PauseMenu` _returnvalue))
    (`UserWidget.AddToViewport` _output_get 0)
    (set `PlayerController.bShowMouseCursor` true (`GameplayStatics.GetPlayerController` 0))))

(fn `f_LockOn`
  (`Controller.SetControlRotation` (`self.GetController`) (`KismetMathLibrary.FindLookAtRotation` (`KismetMathLibrary.MakeVector` (.x (`PlayerCameraManager.GetCameraLocation` (`GameplayStatics.GetPlayerCameraManager` 0))) (.y (`PlayerCameraManager.GetCameraLocation` (`GameplayStatics.GetPlayerCameraManager` 0))) (.z (`PlayerCameraManager.GetCameraLocation` (`GameplayStatics.GetPlayerCameraManager` 0)))) (`KismetMathLibrary.MakeVector` (.x (`self.K2_GetActorLocation` (`self.Target`))) (.y (`self.K2_GetActorLocation` (`self.Target`))) (.z (`self.K2_GetActorLocation` (`self.Target`)))))))

(fn `f_SprintSwitch`
  (params (SprintState :type Boolean))
  (locals (Sprint :type Boolean))
  (bind _charactermovement (`self.CharacterMovement`))
  (bind _charactermovement_2 (`self.CharacterMovement`))
  (set `local.Sprint` SprintState)
  (`/Engine/EditorBlueprintResources/ActorMacros.Switch Has Authority`
    (:`Authority`
      (if (`local.Sprint`)
        (set `CharacterMovementComponent.MaxWalkSpeed` (`self.IncreseSpeed`) _charactermovement_2)
        (set `self.Sprinting` true)
        (else
          (set `CharacterMovementComponent.MaxWalkSpeed` (`self.Speed`) _charactermovement_2)
          (set `self.Sprinting` false)))
      (return))
    (:`Remote`
      (`self.Server_ToggleSprint` (`local.Sprint`))
      (if (`local.Sprint`)
        (set `CharacterMovementComponent.MaxWalkSpeed` (`self.IncreseSpeed`) _charactermovement)
        (else
          (set `CharacterMovementComponent.MaxWalkSpeed` (`self.Speed`) _charactermovement)))
      (return))))

(fn `OnRep_Sprinting`
  (bind _returnvalue (`SkeletalMeshComponent.GetAnimInstance` (`self.Mesh`)))
  (if (`self.Sprinting`)
    (message `/Game/_Main/Interfaces/BPI_PlayerAnimBP.SprintState` _returnvalue true)
    (else
      (message `/Game/_Main/Interfaces/BPI_PlayerAnimBP.SprintState` _returnvalue false))))

(fn `UserConstructionScript`
  (`parent.UserConstructionScript`))