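; Player lock-on targeting component that toggles a camera lock on the closest AI pawn near the owning pawn.
; A sphere overlap, with a debug sphere drawn, gathers candidates and the nearest within range becomes the locked target.
; Interface messages drive the pawn's camera lock and the target's widget.
; A looping timer releases the lock beyond a break distance that is shorter than the search range.
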(event `Initialize`
  (bind _aspawn (cast `Pawn` (`self.GetOwner`)))
  (bind _output_get (set `self.Player Pawn` _aspawn))
  (bind _asplayer_controller (cast `PlayerController` (`Pawn.GetController` _output_get)))
  (set `self.Player Controller` _asplayer_controller))

(event `LockOnTarget`
  (if (not (`self.CurrentTargeting`))
    (`self.FindTargets`)
    (else
      (`self.SwitchCameraLock` false))))

(event `FindTargets`
  (bind _returnvalue (`Actor.K2_GetActorLocation` (`self.Player Pawn`)))
  (bind _outactors (`KismetSystemLibrary.SphereOverlapActors` _returnvalue 1200.0 (`|MakeArray` "ObjectTypeQuery3" :!type "EObjectTypeQuery Enum") "/Game/_Main/AI/AI.AI_C"))
  (`KismetSystemLibrary.DrawDebugSphere` _returnvalue 1000.0 12 (struct :`G` 0.161424 :`B` 1.0 :`A` 1.0) 2.0 5.0)
  (for _array_element _outactors
    (`KismetArrayLibrary.Array_AddUnique` (`self.TargetList`) _array_element))
  (for _array_element_2 (`self.TargetList`)
    (bind _returnvalue_2 (`Actor.GetDistanceTo` (`self.Player Pawn`) _array_element_2))
    (if (< _returnvalue_2 (`self.ClosestDistance`))
      (set `self.ClosestDistance` _returnvalue_2)
      (set `self.LockedTarget` _array_element_2)))
  (set `self.ClosestDistance` 1000.0)
  (`KismetArrayLibrary.Array_Clear` (`self.TargetList`))
  (`self.LockedTarget`
    (:`then`
      (set `self.CurrentTargeting` true)
      (`self.SwitchCameraLock` true)
      (bind _returnvalue_3 (`KismetSystemLibrary.K2_SetTimerDelegate` (delegate `CheckTargetDistance`) 0.25 true))
      (set `self.LockHandle` _returnvalue_3))
    (:`else`)))

(event `CheckTargetDistance`
  (if (> (`Actor.GetDistanceTo` (`self.Player Pawn`) (`self.LockedTarget`)) 500.0)
    (`self.SwitchCameraLock` false)
    (`KismetSystemLibrary.K2_ClearAndInvalidateTimerHandle` (`self.LockHandle`))))

(event `SwitchCameraLock`
  (params (State :type Boolean))
  (bind _player_pawn (`self.Player Pawn`))
  (bind _lockedtarget (`self.LockedTarget`))
  (if State
    (set `self.CurrentTargeting` true)
    (message `/Game/_Main/Interfaces/BPI_PlayerAnimBP.LockCamera` _player_pawn true (`self.LockedTarget`))
    (message `/Game/_Main/Interfaces/BPI_Game.ToggleTargetWidget` _lockedtarget true)
    (else
      (set `self.CurrentTargeting` false)
      (message `/Game/_Main/Interfaces/BPI_PlayerAnimBP.LockCamera` _player_pawn false null)
      (message `/Game/_Main/Interfaces/BPI_Game.ToggleTargetWidget` _lockedtarget false)
      (set `self.LockedTarget` null))))